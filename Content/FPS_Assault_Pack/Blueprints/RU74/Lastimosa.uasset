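; Lastimosa is a first-person pilot character Blueprint that adds double jumping and wallrunning.
; Jumping passes a DoN limit of two into a server launch and montage, reset on landing or wallrun start.
; Capsule overlaps route through server events into a Wallrun graph that checks for airborne contact with "RunWall" actors.
; Its timeline polls player 0's spacebar, toggling zero gravity, a horizontal plane constraint and camera-forward force.
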(event OnComponentBeginOverlap(WallrunCapsuleCollision)
  (params (OverlappedComponent :type Primitive%20Component%20Object%20Reference) (OtherActor :type Actor%20Object%20Reference) (OtherComp :type Primitive%20Component%20Object%20Reference) (OtherBodyIndex :type Integer) (bFromSweep :type Boolean) (SweepResult :type Hit%20Result%20Structure%20%28by%20ref%29))
  (CallFunction|ServerWallrun OtherActor))

(event OnComponentEndOverlap(WallrunCapsuleCollision)
  (params (OverlappedComponent :type Primitive%20Component%20Object%20Reference) (OtherActor :type Actor%20Object%20Reference) (OtherComp :type Primitive%20Component%20Object%20Reference) (OtherBodyIndex :type Integer))
  (CallFunction|ServerEndWallrun OtherActor))

(event Custom|Server%20Jump
  (CallFunction|PilotJump))

(event Custom|Pilot%20Jump
  (Character|LaunchCharacter (Math|Vector|MakeVector 0.0 0.0 (+ (Variables|/Script/Engine.CharacterMovementComponent|GetJumpZVelocity (Variables|Character|GetCharacterMovement)) 1e+02)) false true))

(event Custom|Begin%20Wallrun
  (params (OtherActor :type Actor%20Object%20Reference))
  (|Wallrun OtherActor (stale Custom|EndWallrun OtherActor2)
    (:then_0
      (Utilities|FlowControl|DoN 2) ; enters at Reset
    )))

(event Custom|EndWallrun
  (params (OtherActor2 :type Actor%20Object%20Reference))
  (|Wallrun (stale Custom|Begin%20Wallrun OtherActor) OtherActor2) ; enters at EndOverlap
)

(event Custom|Server%20Wallrun
  (params (OtherActor :type Actor%20Object%20Reference))
  (CallFunction|BeginWallrun OtherActor))

(event Custom|Server%20End%20Wallrun
  (params (OtherActor2 :type Actor%20Object%20Reference))
  (CallFunction|EndWallrun OtherActor2))

(event EventBeginPlay
  (|CallParentFunction) ; This node is disabled and will not be called.\nDrag off pins to build functionality.
)

(event EventTick
  (params (DeltaSeconds :type Float%20%28single-precision%29)))

(event EventJumping
  (Utilities|FlowControl|DoN 2
    (:Exit
      (CallFunction|ServerJump)
      (CallFunction|ServerPlayMontage (Variables|Default|GetMESH_PC_00) "/Game/StylizedModularChar/Animations/Jump_From_Stand_Montage.Jump_From_Stand_Montage" 1.0))))

(event EventOnLanded
  (params (Hit :type Hit%20Result%20Structure%20%28by%20ref%29))
  (Utilities|FlowControl|DoN 2) ; enters at Reset
)

(fn ConstructionScript
  (|CallParentFunction))