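; Child character Blueprint for Hada, a shooter hero with an explosive-pillow ability and a health-triggered caffeine ammo passive.
; The ability plays a melee arm montage, spawns a team-tagged Almohada_Explosiva aimed along a short camera trace through HabilidadHadaRep, then starts its cooldown.
; Salud's low-health and life-lost events call ParcheServer, which uses ParcheCafeina to switch the current weapon's bullet class to caffeine or normal, respectively.
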(event Custom|Habilidad%20Hada%20Rep
  (params (SpawnTransform :type Transform) (Equipo :type Integer))
  (bind _returnvalue (Game|SpawnActorfromClass "/Game/BP/Habilidades/Almohada_Explosiva.Almohada_Explosiva_C" SpawnTransform "Undefined" 0 Equipo self 0)))

(event Custom|Salud%20Baja
  (CallFunction|ParcheServer true (Variables|Default|GetArma%20Actual)))

(event Custom|Perdio%20Vida
  (CallFunction|ParcheServer false (Variables|Default|GetArma%20Actual)))

(event Custom|Parche%20Cafeina
  (params (Activar :type Boolean) (Enumerator :type Armas%20Enum :default "NewEnumerator0"))
  (Development|PrintString (Utilities|String|EnumtoString Enumerator))
  (if Activar
    ;[1 1 1] Cafeina
    (switch Utilities|FlowControl|Switch|SwitchonArmas Enumerator
      (:NewEnumerator0
        (Variables|Default|SetBalasActuales "/Game/BP/Projectiles/Comida_Cafeina.Comida_Cafeina_C"))
      (:NewEnumerator1
        (Variables|Default|SetBalasActuales "/Game/BP/Projectiles/Bala_R47_Cafeina.Bala_R47_Cafeina_C"))
      (:NewEnumerator2
        (Variables|Default|SetBalasActuales "/Game/BP/Projectiles/Bala_Rifle_Cafeina.Bala_Rifle_Cafeina_C"))
      (:NewEnumerator3
        (Variables|Default|SetBalasActuales "/Game/BP/Projectiles/Bala_LimaSMG_Cafeina.Bala_LimaSMG_Cafeina_C"))
      (:NewEnumerator4
        (Variables|Default|SetBalasActuales "/Game/BP/Projectiles/Bala_Escopeta_Cafeina.Bala_Escopeta_Cafeina_C")))
    (else
      ;[1 1 1] Normal
      (switch Utilities|FlowControl|Switch|SwitchonArmas Enumerator
        (:NewEnumerator0
          (Variables|Default|SetBalasActuales "/Game/BP/Projectiles/Comida.Comida_C"))
        (:NewEnumerator1
          (Variables|Default|SetBalasActuales "/Game/BP/Projectiles/Bala_R47.Bala_R47_C"))
        (:NewEnumerator2
          (Variables|Default|SetBalasActuales "/Game/BP/Projectiles/Bala_Rifle.Bala_Rifle_C"))
        (:NewEnumerator3
          (Variables|Default|SetBalasActuales "/Game/BP/Projectiles/Bala_LimaSMG.Bala_LimaSMG_C"))
        (:NewEnumerator4
          (Variables|Default|SetBalasActuales "/Game/BP/Projectiles/Bala_Escopeta.Bala_Escopeta_C"))))))

(event Custom|Parche%20Server
  (params (Activar :type Boolean) (Enumerator :type Armas%20Enum :default "NewEnumerator0"))
  (CallFunction|ParcheCafeina Activar Enumerator))

(event EventBeginPlay
  (bind _salud (Variables|Default|GetSalud))
  (|CallParentFunction)
  (EventDispatchers|BindEventtoSaludBaja _salud (delegate Custom|Salud%20Baja))
  (EventDispatchers|BindEventtoPerdioVida _salud (delegate Custom|Perdio%20Vida)))

(event EventHabilidadPressed
  (bind _first_person_camera (Variables|Default|GetFirst%20Person%20Camera))
  (bind (_start _end) (CallFunction|GetLineTraceDirection 1.5e+02 _first_person_camera))
  (Animation|Montage|PlayMontage (Variables|Default|GetArms) "/Game/FPS_Assault_Pack/Animations/Rifle/A_Arms_Rifle_Melee_Montage.A_Arms_Rifle_Melee_Montage"
    (:then
      (bind _outhit (Collision|LineTraceByChannel _start _end "TraceTypeQuery1" false 0 "None"))
      (CallFunction|HabilidadHadaRep (Math|Transform|MakeTransform _start (Math|Rotator|MakeRotator (.roll (Math|Rotator|FindLookatRotation _start (.traceend _outhit))) (.pitch (Math|Rotator|FindLookatRotation _start (.traceend _outhit))) (.yaw (Math|Rotator|FindLookatRotation _start (.traceend _outhit))))) (Variables|Default|GetEquipo))
      (CallFunction|EjecutarCooldown))))

(fn ConstructionScript
  (|CallParentFunction))