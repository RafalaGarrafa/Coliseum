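; Playable character Bob, whose Q ability spawns a single QBob actor, or removes the active one, with a cooldown.
; A hold-check macro separates tap, which spawns a physics-simulated QBob along a short camera trace, from hold, which previews a hologram and places it without physics on release.
; While holding, a timer loop matches hologram pitch to the camera and mouse wheel adjusts spring-arm distance.
; F fires a shotgun-style spread of Comida projectiles.
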(event OnComponentBeginOverlap(QbobHolograma)
  (params (OverlappedComponent :type Primitive%20Component%20Object%20Reference) (OtherActor :type Actor%20Object%20Reference) (OtherComp :type Primitive%20Component%20Object%20Reference) (OtherBodyIndex :type Integer) (bFromSweep :type Boolean) (SweepResult :type Hit%20Result%20Structure%20%28by%20ref%29)))

(event OnComponentEndOverlap(QbobHolograma)
  (params (OverlappedComponent :type Primitive%20Component%20Object%20Reference) (OtherActor :type Actor%20Object%20Reference) (OtherComp :type Primitive%20Component%20Object%20Reference) (OtherBodyIndex :type Integer)))

(event Custom|Habilidad%20Bob%20Rep
  (params (SpawnTransform :type Transform) (Simulate :type Boolean))
  (bind _returnvalue (Game|SpawnActorfromClass "/Game/BP/Habilidades/QBob.QBob_C" SpawnTransform "Undefined" 0 0))
  (Default|SimulatePhysics _returnvalue Simulate)
  (CallFunction|SpawnQbob :Qbob%20Actual _returnvalue))

(event Custom|Set%20Qbob%20Actual
  (params (Qbob%20Actual :type Q%20Bob%20Object%20Reference))
  (bind _output_get (Variables|Default|SetQbob%20Actual Qbob%20Actual))
  (Development|PrintString (Utilities|GetDisplayName _output_get) true true "(R=0.991543,G=1.000000,B=0.000000,A=1.000000)"))

(event Custom|Desaparecer%20Qbob
  (params (Target :type Q%20Bob%20Object%20Reference))
  (Default|DesaparecerRep Target)
  (Variables|Default|SetQbob%20Actual 0))

(event Custom|Spawn%20Qbob
  (params (SpawnTransform :type Transform) (Qbob%20Actual :type Q%20Bob%20Object%20Reference))
  (CallFunction|SetQbobActual Qbob%20Actual)
  (Development|PrintString (Utilities|GetDisplayName Qbob%20Actual) true true "(R=1.000000,G=0.000000,B=0.017764,A=1.000000)"))

(event Custom|Reset%20Habilidad%20Pressed
  (bind (_start _end _simulate) (CallFunction|IsHolodingQ?))
  (Utilities|FlowControl|DoOnce false) ; enters at Reset
)

(event EventBeginPlay
  (|CallParentFunction)
  (EventDispatchers|BindEventtoAbilityReseted (delegate Custom|Reset%20Habilidad%20Pressed)))

(event EventHabilidadReleased
  (bind (_start _end _simulate) (CallFunction|IsHolodingQ?))
  (Utilities|FlowControl|DoOnce false
    (:Completed
      (Utilities|CheckHold 0.5 true) ; enters at Released
    )))

(event EventDespawn
  (bind _qbob_actual (Variables|Default|GetQbob%20Actual)
    (:then
      (CallFunction|DesaparecerQbob _qbob_actual))
    (:else)))

(event EventHabilidadPressed
  (bind (_start _end _simulate) (CallFunction|IsHolodingQ?))
  (Utilities|CheckHold 0.5 true
    (:Held
      (Variables|Default|GetQbob%20Actual
        (:then)
        (:else
          (Variables|Default|SetTappedQ false)
          (Rendering|SetVisibility (Variables|Default|GetQbobHolograma) true false)
          (Utilities|FlowControl|Sequence
            (:then_0
              (goto _label Open))
            (:then_1
              (Utilities|FlowControl|Gate true :!label _label
                (:Exit
                  (CallFunction|SetQBobHRot)
                  (Variables|Default|SetHoldingQ true)
                  (Utilities|FlowControl|RetriggerableDelay 0.05)
                  (goto _label))))))))
    (:Tap
      _)
    (:Button%20Released
      (Variables|/Script/Engine.SpringArmComponent|SetTargetArmLength (Variables|Default|GetSpringArm2) 7e+02)
      (Variables|Default|SetHoldingQ false)
      (Utilities|FlowControl|Sequence
        (:then_0
          _)
        (:then_1
          (goto _label Close)))))
  (Rendering|SetVisibility (Variables|Default|GetQbobHolograma) false false)
  (CallFunction|EjecutarCooldown)
  (Animation|Montage|PlayMontage (Variables|Default|GetArms) "/Game/FPS_Assault_Pack/Animations/Rifle/A_Arms_Rifle_Melee_Montage.A_Arms_Rifle_Melee_Montage"
    (:then
      (Development|PrintString (Utilities|GetDisplayName (Variables|Default|GetQbob%20Actual)))
      (Development|PrintString "Habilidad Bob")
      (bind _qbob_actual (Variables|Default|GetQbob%20Actual)
        (:then
          (CallFunction|DesaparecerQbob _qbob_actual)
          (CallFunction|CambiarIcono "/Game/MiCosas/Texturas/Habilidades/BobQ.BobQ"))
        (:else
          (CallFunction|CambiarIcono "/Game/MiCosas/Texturas/Habilidades/BobQVacio.BobQVacio")
          (bind _outhit (Collision|LineTraceByChannel (Transformation|GetWorldLocation (Variables|Default|GetFirst%20Person%20Camera)) _end "TraceTypeQuery1" false 0 "None"))
          (if (.bblockinghit _outhit)
            (CallFunction|HabilidadBobRep (CallFunction|MakeQbobTransform _start (.impactpoint _outhit)) _simulate)
            (else
              (CallFunction|HabilidadBobRep (CallFunction|MakeQbobTransform _start (.traceend _outhit)) _simulate))))))))

(event Input|MouseEvents|MouseWheelUp
  (params (Key :type Key%20Structure :default "None"))
  (:Pressed
    (CallFunction|SetTargetArmL 5e+01)))

(event Input|KeyboardEvents|F
  (params (Key :type Key%20Structure :default "None"))
  (:Pressed
    (if (Utilities|Enum|NotEqual(Enum) (Variables|Default|GetArma%20Actual) "NewEnumerator0")
      (Utilities|FlowControl|DoOnce false :!label _label
        (:Completed
          (bind _returnvalue (Animation|Montage|MontagePlay (Components|SkeletalMesh|GetAnimInstance (Variables|Default|GetArms)) "/Game/FPS_Assault_Pack/Animations/Rifle/A_Arms_Rifle_Grenade_Montage.A_Arms_Rifle_Grenade_Montage" 1.0 "MontageLength" 0.18 true))
          (Utilities|FlowControl|Delay (- _returnvalue 1.0))
          (bind _transformsescopeta1 (CallFunction|MakeLineTrace "NewEnumerator4" 3))
          (for _array_element _transformsescopeta1
            (CallFunction|SpawnProejctileServer "/Game/BP/Projectiles/Comida.Comida_C" _array_element false))
          (Utilities|FlowControl|Delay 0.5)
          (goto _label Reset))))))

(event Input|MouseEvents|MouseWheelDown
  (params (Key :type Key%20Structure :default "None"))
  (:Pressed
    (CallFunction|SetTargetArmL -5e+01)))

(fn ConstructionScript
  (|CallParentFunction))

(fn IsHolodingQ?
  (bind _first_person_camera (Variables|Default|GetFirst%20Person%20Camera))
  (bind (_start _end) (CallFunction|GetLineTraceDirection 2.5e+02 _first_person_camera))
  (if (Variables|Default|GetTappedQ)
    (return _start _end true)
    (else
      (return (.Start (CallFunction|GetLineTraceDirection 0.0 _first_person_camera)) (Transformation|GetWorldLocation (Variables|Default|GetQBobSpawnLoc)) false))))

(fn CambiarIcono
  (params (Texture :type Texture%202D%20Object%20Reference))
  (Class|WidgetBlueprintLibrary|SetBrushResourcetoTexture (Variables|/Game/BP/Salud.Salud_C|GetIcono_Habilidad (Variables|Default|GetSalud)) Texture)
  (CallFunction|SetAbilityIcon (Variables|Default|GetHUD)))

(fn SetQBobHRot
  (Transformation|SetRelativeRotation (Variables|Default|GetSceneQBHRot) (Math|Rotator|MakeRotator 0.0 (.pitch (Transformation|GetWorldRotation (Variables|Default|GetFirst%20Person%20Camera))) 0.0) false false))

(fn ColorQbobHolo
  (params (Color :type Linear%20Color%20Structure) (Check%20If%20Holding :type Boolean) (CanSpawn :type Boolean))
  (if Check%20If%20Holding
    (if (Variables|Default|GetHoldingQ)
      (Rendering|Material|SetVectorParameterValue (Variables|Default|GetQbobHolo_MI) "Color" Color :!class /Script/Engine.MaterialInstanceDynamic :!label _label)
      (Variables|Default|SetCanSpawn CanSpawn))
    (else
      (goto _label))))

(fn MakeQbobTransform
  (params (Start :type Vector%20%28by%20ref%29) (Target :type Vector%20%28by%20ref%29))
  (return (Math|Transform|MakeTransform Target (Math|Rotator|MakeRotator 0.0 0.0 (.yaw (Math|Rotator|FindLookatRotation Start Target))))))

(fn SetTargetArmL
  (params (Increment :type Float%20%28single-precision%29))
  (if (Variables|Default|GetHoldingQ)
    (Variables|/Script/Engine.SpringArmComponent|SetTargetArmLength (Variables|Default|GetSpringArm2) (Math|Float|Clamp(Float) (+ (Variables|/Script/Engine.SpringArmComponent|GetTargetArmLength (Variables|Default|GetSpringArm2)) Increment) (LocalVariables|GetMin%20Lenght) (LocalVariables|GetMax%20Lenght)))
    (return)))