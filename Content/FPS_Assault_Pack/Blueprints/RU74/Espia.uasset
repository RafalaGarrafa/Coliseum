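; Spy (Espia) player character Blueprint with a special ability and an explosive on death.
; Pressing the ability plays a rifle melee montage on the arms, spawns a Revelador at the start of a short camera trace, aimed along it, then starts the cooldown.
; Morir extends the parent's death logic by spawning an ExplosivoEspia owned by the player.
; Debug explosive and ground-snapped Revelador placement chains are left unconnected.
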(event Custom|Spawn%20Revelador
  (params (SpawnTransform :type Transform))
  (Game|SpawnActorfromClass "/Game/BP/Habilidades/Revelador.Revelador_C" SpawnTransform "Undefined" 0 self 0))

(event Custom|Spawn%20Explosion%20Espia
  (params (SpawnTransform :type Transform))
  (Game|SpawnActorfromClass "/Game/BP/Habilidades/ExplosivoEspia.ExplosivoEspia_C" SpawnTransform "Undefined" 0 self 0))

(event Custom|Spawn%20Pluma%20DEBUG
  (params (SpawnTransform :type Transform))
  (Game|SpawnActorfromClass "/Game/BP/Habilidades/ExplosivoEspia.ExplosivoEspia_C" SpawnTransform "Undefined" 0 0 0))

(event EventBeginPlay
  (|CallParentFunction) ; This node is disabled and will not be called.\nDrag off pins to build functionality.
)

(event Collision|EventActorBeginOverlap
  (params (OtherActor :type Actor%20Object%20Reference)))

(event EventTick
  (params (DeltaSeconds :type Float%20%28single-precision%29)))

(event EventHabilidadPressed
  (bind _first_person_camera (Variables|Default|GetFirst%20Person%20Camera))
  (bind (_start _end) (CallFunction|GetLineTraceDirection 2.5e+02 _first_person_camera))
  (Animation|Montage|PlayMontage (Variables|Default|GetArms) "/Game/FPS_Assault_Pack/Animations/Rifle/A_Arms_Rifle_Melee_Montage.A_Arms_Rifle_Melee_Montage"
    (:then
      (bind _outhit (Collision|LineTraceByChannel _start _end "TraceTypeQuery1" false 0 "None"))
      (CallFunction|SpawnRevelador (Math|Transform|MakeTransform _start (Math|Rotator|FindLookatRotation _start (.traceend _outhit))))
      (CallFunction|EjecutarCooldown))))

(event EventMorir
  (|CallParentFunction)
  (CallFunction|SpawnExplosionEspia (Transformation|GetActorTransform)))

(event Input|KeyboardEvents|X
  (params (Key :type Key%20Structure :default "None")))

(fn ConstructionScript
  (|CallParentFunction))